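; VR player pawn that samples headset pose and turns off capsule physics where it lacks network authority.
; Tick calls HMD every tenth of a second to combine device pose with the camera transform and pass it to SeverHMD.
; SeverHMD stores the pose and calls ClientHMD, which, if locally controlled, places Arrow at the capsule with the headset rotation.
; The stored HMD location is not read here.
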(event `self.ReceiveBeginPlay`
  (`/Engine/EditorBlueprintResources/ActorMacros.Switch Has Authority`
    (:`Remote`
      (`PrimitiveComponent.SetSimulatePhysics` (`self.Capsule`) false))))

(event `HMD`
  (bind (_devicerotation _deviceposition) (`HeadMountedDisplayFunctionLibrary.GetOrientationAndPosition`))
  (`self.Sever HMD` (`KismetMathLibrary.MakeRotator` (.roll _devicerotation) (* (.pitch _devicerotation) 1.0) (+ (.yaw _devicerotation) (.yaw (`SceneComponent.K2_GetComponentRotation` (`self.Camera`))))) (`KismetMathLibrary.TransformLocation` (`SceneComponent.K2_GetComponentToWorld` (`self.Camera`)) _deviceposition)))

(event `Sever HMD`
  (params (Rotation :type "Rotator Structure") (Position :type "Vector Structure"))
  (set `self.HMDRotation` Rotation)
  (set `self.HMDLocation` Position)
  (`self.Client HMD`))

(event `Client HMD`
  (if (`self.IsLocallyControlled` self)
    (`SceneComponent.K2_SetWorldTransform` (`self.Arrow`) (`KismetMathLibrary.MakeTransform` (`SceneComponent.K2_GetComponentLocation` (`self.Capsule`)) (`self.HMDRotation`)) false false)))

(event `self.ReceiveTick`
  (params (DeltaSeconds :type "Float (single-precision)"))
  (bind _returnvalue (- (`self.Timer`) DeltaSeconds))
  (`|ExecutionSequence`
    (:`then_0`
      (if (<= _returnvalue 0.0)
        (set `self.Timer` 0.1)
        (`self.HMD`)
        (else
          (set `self.Timer` _returnvalue))))))

(fn `UserConstructionScript`)