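; DummyPawn is a pawn that hosts a MenuWidget component and lets the player click UI through a WidgetInteraction component.
; The Select input action presses and releases a simulated left mouse button on the interaction component.
; Functions post a widget to MenuWidget and show it, or return the current one.
; RemoveFromMenuWidget checks that the target is active, but sets visibility to true rather than hiding or clearing it.
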(event `InputAction|Select`
  (params (Key :type "Key Structure"))
  (:`Pressed`
    (`WidgetInteractionComponent.PressPointerKey` (`self.WidgetInteraction`) "LeftMouseButton"))
  (:`Released`
    (`WidgetInteractionComponent.ReleasePointerKey` (`self.WidgetInteraction`) "LeftMouseButton")))

(fn `GetCurrentMenuWidget`
  (returns (CurrentWidget :type "Widget Object Reference"))
  (return (`WidgetComponent.GetUserWidgetObject` (`self.MenuWidget`))))

(fn `PostToMenuWidget`
  (params (TargetWidget :type "Widget Object Reference"))
  (bind _menuwidget (`self.MenuWidget`))
  (`WidgetComponent.SetWidget` _menuwidget (cast `UserWidget` TargetWidget :!pure true))
  (`SceneComponent.SetVisibility` _menuwidget true false))

(fn `RemoveFromMenuWidget`
  (params (TargetWidget :type "Widget Object Reference"))
  (bind _menuwidget (`self.MenuWidget`))
  (if (== TargetWidget (`WidgetComponent.GetUserWidgetObject` _menuwidget))
    (`SceneComponent.SetVisibility` _menuwidget true false)
    (else
      (`KismetSystemLibrary.PrintString` "This widget is not active!!!"))))

(fn `UserConstructionScript`)